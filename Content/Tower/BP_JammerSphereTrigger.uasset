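; BP_JammerSphereTrigger is a short-lived expanding jammer sphere that destroys radio sphere triggers it overlaps.
; Each Tick it advances Lifetime, polls the sphere's overlapping actors to destroy BP_RadioSphereTrigger instances, then lerps the sphere's scale from zero to SphereFinalSize over TimeToMaxScale.
; It destroys itself once Lifetime exceeds LifetimeMax.
; The node capturing SphereFinalSize from the sphere's scale is unconnected, so the variable's stored value is used.
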(event EventBeginPlay)

(event Collision|EventActorBeginOverlap
  (params (OtherActor :type Actor%20Object%20Reference)))

(event EventTick
  (params (DeltaSeconds :type Float%20%28single-precision%29))
  (CallFunction|IncreaseLifetime DeltaSeconds)
  (CallFunction|DestroyOverlappingRadioTowers)
  (CallFunction|GrowObjects)
  (if (> (Variables|Default|GetLifetime) (Variables|Default|GetLifetime_Max))
    (Actor|DestroyActor)))

(fn ConstructionScript)

(fn DestroyOverlappingRadioTowers
  (for _array_element (Collision|GetOverlappingActors (Variables|Default|GetSphere) 0 :!class /Script/Engine.PrimitiveComponent)
    (bind _asbp_radio_sphere_trigger (Utilities|Casting|CastToBP_RadioSphereTrigger _array_element))
    (Actor|DestroyActor _asbp_radio_sphere_trigger)))

(fn IncreaseLifetime
  (params (DeltaSeconds :type Float%20%28single-precision%29))
  (Variables|Default|SetLifetime (+ (Variables|Default|GetLifetime) DeltaSeconds)))

(fn GrowObjects
  (if (not (> (Variables|Default|GetLifetime) (Variables|Default|GetTimeToMaxScale)))
    (Transformation|SetWorldScale3D (Variables|Default|GetSphere) (Math|Vector|Lerp(Vector) "0, 0, 0" (Variables|Default|GetSphereFinalSize) (/ (Variables|Default|GetLifetime) (Variables|Default|GetTimeToMaxScale))))))