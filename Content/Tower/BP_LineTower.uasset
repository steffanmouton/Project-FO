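; BP_LineTower is a tower actor that stretches its Cube component along Z into a long line over time.
; BeginPlay stores the Cube's starting world scale, and each Tick builds the target scale, accumulates Lifetime and passes it to LineGrowthFunction.
; That function linearly interpolates from start to target scale, with ScaleFactorZ as the final Z scale, and stops updating once Lifetime exceeds TimeToMaxScaleS.
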(event EventBeginPlay
  (Variables|Default|SetScaleStart (Transformation|GetWorldScale (Variables|Default|GetCube))))

(event EventTick
  (params (DeltaSeconds :type Float%20%28single-precision%29))
  (bind _scalestart (Variables|Default|GetScaleStart))
  ;[1 1 1] Set the Scale Vector, Increment Lifetime, Call Line Growth
  (Variables|Default|SetScaleMax (Math|Vector|MakeVector (.x _scalestart) (.y _scalestart) (Variables|Default|GetScaleFactor_Z)))
  (bind _output_get (Variables|Default|SetLifetime (+ (Variables|Default|GetLifetime) DeltaSeconds)))
  (CallFunction|LineGrowthFunction _output_get))

(fn ConstructionScript)

(fn LineGrowthFunction
  (params (Lifetime :type Float%20%28single-precision%29))
  (bind _timetomaxscale_s (Variables|Default|GetTimeToMaxScale_S))
  ;[1 1 1] Scales the Cube object out into a long line over time, if still in growth time
  (if (not (> (Variables|Default|GetLifetime) _timetomaxscale_s))
    (Transformation|SetWorldScale3D (Variables|Default|GetCube) (Math|Vector|Lerp(Vector) (Variables|Default|GetScaleStart) (Variables|Default|GetScaleMax) (/ (Variables|Default|GetLifetime) _timetomaxscale_s)))))