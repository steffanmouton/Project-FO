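; Tower actor whose signal sphere grows over time after play begins, according to its power level.
; Tick accumulates lifetime and passes it to SphereGrowthFunction, which lerps the sphere's world scale from its starting value.
; Each S, M or L level has its own growth time, after which scaling stops.
; Level M targets the small maximum scale, MaxScaleS, rather than a medium one.
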(event EventBeginPlay
  (Variables|Default|SetStartScale (Transformation|GetWorldScale (Variables|Default|GetSignalSphere))))

(event EventTick
  (params (DeltaSeconds :type Float%20%28single-precision%29))
  (bind _output_get (Variables|Default|SetLifetime (+ (Variables|Default|GetLifetime) DeltaSeconds)))
  (CallFunction|SphereGrowthFunction _output_get))

(fn ConstructionScript)

(fn SphereGrowthFunction
  (params (Lifetime :type Float%20%28single-precision%29))
  (switch string (Variables|Default|GetPowerLevel)
    (:S
      (if (not (> (Variables|Default|GetLifetime) (Variables|Default|GetTimeToMaxScale_S)))
        (Transformation|SetWorldScale3D (Variables|Default|GetSignalSphere) (Math|Vector|Lerp(Vector) (Variables|Default|GetStartScale) (Variables|Default|GetMaxScale_S) (/ (Variables|Default|GetLifetime) (Variables|Default|GetTimeToMaxScale_S))))))
    (:M
      (if (not (> (Variables|Default|GetLifetime) (Variables|Default|GetTimeToMaxScale_M)))
        (Transformation|SetWorldScale3D (Variables|Default|GetSignalSphere) (Math|Vector|Lerp(Vector) (Variables|Default|GetStartScale) (Variables|Default|GetMaxScale_S) (/ (Variables|Default|GetLifetime) (Variables|Default|GetTimeToMaxScale_M))))))
    (:L
      (if (not (> (Variables|Default|GetLifetime) (Variables|Default|GetTimeToMaxScale_L)))
        (Transformation|SetWorldScale3D (Variables|Default|GetSignalSphere) (Math|Vector|Lerp(Vector) (Variables|Default|GetStartScale) (Variables|Default|GetMaxScale_L) (/ (Variables|Default|GetLifetime) (Variables|Default|GetTimeToMaxScale_L))))))))