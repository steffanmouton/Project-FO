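; BP_RadioLine is a tower-related actor that destroys overlapping Sedan actors tagged "SphereTower".
; Each Tick it queries its static mesh for overlapping actors of the Sedan class and checks their tags, polling rather than using overlap events.
; It also accumulates a Lifetime counter from delta time, which nothing in this Blueprint reads beyond that increment.
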(event EventBeginPlay)

(event EventTick
  (params (DeltaSeconds :type Float%20%28single-precision%29))
  (CallFunction|IncreaseLifetime DeltaSeconds)
  (for _array_element (Collision|GetOverlappingActors (Variables|Default|GetStaticMesh) "/Game/VehicleBP/Sedan/Sedan.Sedan_C" :!class /Script/Engine.PrimitiveComponent)
    (for _array_element_2 (Variables|/Script/Engine.Actor|GetTags _array_element)
      (if (Utilities|Name|Equal(Name) _array_element_2 "SphereTower")
        (Actor|DestroyActor _array_element)))))

(fn ConstructionScript)

(fn IncreaseLifetime
  (params (DeltaSeconds :type Float%20%28single-precision%29))
  (Variables|Default|SetLifetime (+ (Variables|Default|GetLifetime) DeltaSeconds)))